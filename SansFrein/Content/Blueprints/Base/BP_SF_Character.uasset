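; BP_SF_Character is a player character that handles look input, tracks a score and creates its HUD on BeginPlay.
; Mouse look feeds controller yaw and pitch, and its X value also drives sideways movement through the Move function.
; IA_Move calls Move with zero values, so it adds no movement.
; AddScore increases the score, and anything overlapping the Box component is destroyed.
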(event OnComponentBeginOverlap(Box)
  (params (OverlappedComponent :type Primitive%20Component%20Object%20Reference) (OtherActor :type Actor%20Object%20Reference) (OtherComp :type Primitive%20Component%20Object%20Reference) (OtherBodyIndex :type Integer) (bFromSweep :type Boolean) (SweepResult :type Hit%20Result%20Structure%20%28by%20ref%29))
  (Actor|DestroyActor OtherActor))

(event Custom|AddScore
  (params (Score :type Integer))
  ;[0.15 0.15 0.15 0.5] Add Score To Player
  (Variables|Default|SetScore (+ Score (Variables|Default|GetScore))))

(event Input|EnhancedActionEvents|EnhancedInputActionIA_MouseLook
  (params (ActionValue :type Vector%202D%20Structure) (ElapsedSeconds :type Float%20%28double-precision%29) (TriggeredSeconds :type Float%20%28double-precision%29) (InputAction :type Input%20Action%20Object%20Reference :default "/Game/Input/IA_MouseLook.IA_MouseLook"))
  (CallFunction|Aim (.x ActionValue) (.y ActionValue))
  (CallFunction|Move (.x ActionValue) 0.0))

(event Input|EnhancedActionEvents|EnhancedInputActionIA_Move
  (params (ActionValue :type Vector%202D%20Structure) (ElapsedSeconds :type Float%20%28double-precision%29) (TriggeredSeconds :type Float%20%28double-precision%29) (InputAction :type Input%20Action%20Object%20Reference :default "/Game/Input/IA_Move.IA_Move"))
  (CallFunction|Move 0.0 0.0))

(event Collision|EventActorBeginOverlap
  (params (OtherActor :type Actor%20Object%20Reference)))

(event EventTick
  (params (DeltaSeconds :type Float%20%28single-precision%29)))

(event EventBeginPlay
  (bind _returnvalue (UserInterface|CreateWidget "/Game/HUD.HUD_C"))
  (UserInterface|Viewport|AddtoViewport _returnvalue 0))

(fn ConstructionScript)

(fn Aim
  (params (Yaw :type Float%20%28double-precision%29) (Pitxh :type Float%20%28double-precision%29))
  (Pawn|Input|AddControllerYawInput Yaw)
  (Pawn|Input|AddControllerPitchInput Pitxh))

(fn Move
  (params (Left%20/%20Right :type Float%20%28double-precision%29) (Forward%20/%20Backward :type Float%20%28double-precision%29))
  (Pawn|Input|AddMovementInput (Transformation|GetActorRightVector) Left%20/%20Right false)
  (Pawn|Input|AddMovementInput (Transformation|GetActorForwardVector) Forward%20/%20Backward false))