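; Terrain Blueprint that randomly dresses its four zones with scenery and obstacles on BeginPlay.
; Left and right zones make a few attempts to attach random EnvList meshes to random child boxes, skipping an immediate repeat.
; Middle and back zones attach only one random ObsList mesh each, as later loop passes place nothing once the current box is set.
; Those obstacle boxes become visible and block WorldDynamic.
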(event Collision|EventActorBeginOverlap
  (params (OtherActor :type Actor%20Object%20Reference)))

(event EventTick
  (params (DeltaSeconds :type Float%20%28single-precision%29)))

(event EventBeginPlay
  (CallFunction|SpawnLeftZone)
  (CallFunction|SpawnRightZone)
  (CallFunction|SpawnMiddleZone)
  (CallFunction|SpawnBackZone))

(fn ConstructionScript)

(fn Translate)

(fn SpawnLeftZone
  (for _index (range 0 (Math|Random|RandomIntegerinRange 1 2))
    (Development|PrintString (Utilities|String|ToString(Integer) _index))
    (bind _asbox_collision (Utilities|Casting|CastToBoxComponent (.OutItem (Utilities|Array|Random (Components|GetChildrenComponents (Variables|Default|GetLeftZone) false)))))
    (Utilities|IsValid (Variables|Default|GetCurrentLeftZoneEl)
      (:Is%20Valid
        (if (!= _asbox_collision (Variables|Default|GetCurrentLeftZoneEl))
          (Variables|Default|SetCurrentLeftZoneEl _asbox_collision :!label _label)
          (bind _returnvalue (AddComponent|AddStaticMeshComponent false (Math|Transform|MakeTransform (Math|Vector|MakeVector 0.0 0.0 -565.0) "0, 0, 0" "0.100000,0.100000,1.500000")))
          (Transformation|AttachComponentToComponent _returnvalue (Variables|Default|GetCurrentLeftZoneEl) "None" "KeepRelative" "KeepRelative" "KeepRelative" false)
          (Components|StaticMesh|SetStaticMesh _returnvalue (.OutItem (Utilities|Array|Random (Variables|Default|GetEnvList))))
          (else
            (Development|PrintString "EQUAL ZONE !"))))
      (:Is%20Not%20Valid
        (goto _label))))
  (Development|PrintString "Left Env Spawned"))

(fn SpawnRightZone
  (for _index (range 0 (Math|Random|RandomIntegerinRange 1 2))
    (Development|PrintString (Utilities|String|ToString(Integer) _index))
    (bind _asbox_collision (Utilities|Casting|CastToBoxComponent (.OutItem (Utilities|Array|Random (Components|GetChildrenComponents (Variables|Default|GetRightZone) false)))))
    (Utilities|IsValid (Variables|Default|GetCurrentRightZoneEl)
      (:Is%20Valid
        (if (!= _asbox_collision (Variables|Default|GetCurrentRightZoneEl))
          (Variables|Default|SetCurrentRightZoneEl _asbox_collision :!label _label)
          (bind _returnvalue (AddComponent|AddStaticMeshComponent false (Math|Transform|MakeTransform (Math|Vector|MakeVector 0.0 0.0 -565.0) "0, 0, 0" "0.100000,0.100000,1.500000")))
          (Transformation|AttachComponentToComponent _returnvalue (Variables|Default|GetCurrentRightZoneEl) "None" "KeepRelative" "KeepRelative" "KeepRelative" false)
          (Components|StaticMesh|SetStaticMesh _returnvalue (.OutItem (Utilities|Array|Random (Variables|Default|GetEnvList))))
          (else
            (Development|PrintString "EQUAL ZONE !"))))
      (:Is%20Not%20Valid
        (goto _label))))
  (Development|PrintString "Right Env Spawned"))

(fn SpawnMiddleZone
  (for _index (range 0 (Math|Random|RandomIntegerinRange 1 2))
    (Development|PrintString (Utilities|String|ToString(Integer) _index))
    (bind _asbox_collision (Utilities|Casting|CastToBoxComponent (.OutItem (Utilities|Array|Random (Components|GetChildrenComponents (Variables|Default|GetMiddleZone) false)))))
    (Utilities|IsValid (Variables|Default|GetCurrentMiddleZoneObs)
      (:Is%20Valid
        (if (not (!= _asbox_collision (Variables|Default|GetCurrentMiddleZoneObs)))
          (Development|PrintString "EQUAL ZONE !")))
      (:Is%20Not%20Valid
        (Variables|Default|SetCurrentMiddleZoneObs _asbox_collision)
        (bind _returnvalue (AddComponent|AddStaticMeshComponent false (Math|Transform|MakeTransform (Math|Vector|MakeVector 0.0 0.0 -596.0) "0, 0, 0" "0.100000,0.100000,1.500000")))
        (Transformation|AttachComponentToComponent _returnvalue (Variables|Default|GetCurrentMiddleZoneObs) "None" "KeepRelative" "KeepRelative" "KeepRelative" false)
        (Components|StaticMesh|SetStaticMesh _returnvalue (.OutItem (Utilities|Array|Random (Variables|Default|GetObsList))))
        (Development|SetHiddeninGame (Variables|Default|GetCurrentMiddleZoneObs) false false)
        (Collision|SetCollisionEnabled (Variables|Default|GetCurrentMiddleZoneObs) "QueryAndPhysics")
        (Collision|SetCollisionResponsetoChannel (Variables|Default|GetCurrentMiddleZoneObs) "ECC_WorldDynamic" "ECR_Block"))))
  (Development|PrintString "Middle Obs Spawned"))

(fn SpawnBackZone
  (for _index (range 0 (Math|Random|RandomIntegerinRange 1 2))
    (Development|PrintString (Utilities|String|ToString(Integer) _index))
    (bind _asbox_collision (Utilities|Casting|CastToBoxComponent (.OutItem (Utilities|Array|Random (Components|GetChildrenComponents (Variables|Default|GetBackZone) false)))))
    (Utilities|IsValid (Variables|Default|GetCurrentBackZoneObs)
      (:Is%20Valid
        (if (not (!= _asbox_collision (Variables|Default|GetCurrentBackZoneObs)))
          (Development|PrintString "EQUAL ZONE !")))
      (:Is%20Not%20Valid
        (Variables|Default|SetCurrentBackZoneObs _asbox_collision)
        (bind _returnvalue (AddComponent|AddStaticMeshComponent false (Math|Transform|MakeTransform (Math|Vector|MakeVector 0.0 0.0 -596.0) "0, 0, 0" "0.100000,0.100000,1.500000")))
        (Transformation|AttachComponentToComponent _returnvalue (Variables|Default|GetCurrentBackZoneObs) "None" "KeepRelative" "KeepRelative" "KeepRelative" false)
        (Components|StaticMesh|SetStaticMesh _returnvalue (.OutItem (Utilities|Array|Random (Variables|Default|GetObsList))))
        (Development|SetHiddeninGame (Variables|Default|GetCurrentBackZoneObs) false false)
        (Collision|SetCollisionEnabled (Variables|Default|GetCurrentBackZoneObs) "QueryAndPhysics")
        (Collision|SetCollisionResponsetoChannel (Variables|Default|GetCurrentBackZoneObs) "ECC_WorldDynamic" "ECR_Block"))))
  (Development|PrintString "Back Obs Spawned"))