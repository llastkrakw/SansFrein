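; Player-driven physics hovercar that floats on four hover points and steers through Enhanced Input.
; Each tick, downward traces at the points apply lift inversely proportional to ground distance, followed by linear and angular damping.
; IA_Accelerate applies yaw torque and thrust from forces precomputed using mass and inertia; airborne state weakens forward thrust and linear damping.
; When TurnOn is set, LimitRotation pins pitch and roll, as its clamp bounds are identical.
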(event Custom|Initialize%20Forces
  (ForcesCalculations|CalculateHoverForce)
  (CallFunction|CalculateMovementForce))

(event Input|EnhancedActionEvents|EnhancedInputActionIA_Accelerate
  (params (ActionValue :type Vector%202D%20Structure) (ElapsedSeconds :type Float%20%28double-precision%29) (TriggeredSeconds :type Float%20%28double-precision%29) (InputAction :type Input%20Action%20Object%20Reference :default "/Game/Inputs/IA_Accelerate.IA_Accelerate"))
  (CallFunction|ApplyMovement ActionValue))

(event EventBeginPlay
  (bind _returnvalue (Game|GetPlayerController 0))
  (Input|EnableInput _returnvalue)
  (Input|AddMappingContext (PlayerController|LocalPlayerSubsystems|GetEnhancedInputLocalPlayerSubsystem _returnvalue) "/Game/Inputs/IC_Vehicle.IC_Vehicle" 0 "(bIgnoreAllPressedKeysUntilRelease=True,bForceImmediately=False,bNotifyUserSettings=False)")
  (Initialization|InitializeHover)
  (CallFunction|InitializeForces))

(event EventTick
  (params (DeltaSeconds :type Float%20%28single-precision%29))
  (CallFunction|GetGrounded)
  (Hover|ApplyHoverForce)
  (Stabilization|ApplyLinearDamping)
  (Stabilization|ApplyAngularDamping)
  (Stabilization|LimitRotation))

(fn ConstructionScript)

(fn InitializeHover
  (Variables|HoverShip|SetHover_Points (Utilities|Array|MakeArray (Variables|Default|GetHover_Point_2) (Variables|Default|GetHover_Point_3) (Variables|Default|GetHover_Point_4) (Variables|Default|GetHover_Point_1))))

(fn CalculateHoverForce
  (Variables|Hover|SetHover_Force (* (* (Physics|GetMass (Variables|Default|GetSM_Ship)) (Variables|Hover|GetHover_Acceleration)) 1.5e+02)))

(fn ApplyHoverForce
  (for _array_element (Variables|HoverShip|GetHover_Points)
    (bind (_outhit _returnvalue) (Collision|LineTraceByChannel (Transformation|GetWorldLocation _array_element) (+ (Transformation|GetWorldLocation _array_element) (* (Math|Vector|MakeVector 0.0 0.0 -1.0) (Variables|Hover|GetHover_Distance))) "TraceTypeQuery1" false 0 "ForDuration" true "(R=1.000000,G=0.000000,B=0.000000,A=1.000000)" "(R=0.000000,G=1.000000,B=0.000000,A=1.000000)" 0.0))
    (if _returnvalue
      (Class|PrimitiveComponent|AddForceatLocation (Variables|Default|GetSM_Ship) (* (Math|Vector|GetUpVector (Variables|Default|GetSM_Ship)) (/ (Variables|Hover|GetHover_Force) (.Distance (Collision|BreakHitResult _outhit)))) (Transformation|GetWorldLocation _array_element) "None"))))

(fn GetGrounded
  (bind _sm_ship (Variables|Default|GetSM_Ship))
  (bind _returnvalue (Transformation|GetWorldLocation _sm_ship))
  (bind _returnvalue_2 (Collision|LineTraceByChannel _returnvalue (+ _returnvalue (* (Math|Vector|MakeVector 0.0 0.0 -1.0) (Variables|HoverShip|GetCheckGroundDistance))) "TraceTypeQuery1" false 0 "ForDuration" true "(R=0.000000,G=0.231763,B=1.000000,A=1.000000)" "(R=0.000000,G=1.000000,B=0.000000,A=1.000000)" 0.0))
  (Variables|HoverShip|SetIs_Grounded? _returnvalue_2))

(fn ApplyLinearDamping
  (bind _linear_damping_force (Variables|Stabilization|GetLinear_Damping_Force))
  (Physics|AddForce (Variables|Default|GetSM_Ship) (* (* (Transformation|GetComponentVelocity (Variables|Default|GetSM_Ship)) -1.0) (Math|Float|SelectFloat _linear_damping_force (/ _linear_damping_force 4.0) (Variables|HoverShip|GetIs_Grounded?))) "None" false))

(fn ApplyAngularDamping
  (bind _sm_ship (Variables|Default|GetSM_Ship))
  (Class|PrimitiveComponent|AddTorqueinRadians (Variables|Default|GetSM_Ship) (* (* (Class|PrimitiveComponent|GetPhysicsAngularVelocityinRadians _sm_ship "None") -1.0) (* (Class|PrimitiveComponent|GetInertiaTensor _sm_ship "None") (Variables|Stabilization|GetAngular_Damping_Force))) "None" false))

(fn LimitRotation
  (bind _sm_ship (Variables|Default|GetSM_Ship))
  (bind _min_rotation_angle (Variables|Stabilization|GetMin_Rotation_Angle))
  (bind _min_rotation_angle_2 (Variables|Stabilization|GetMin_Rotation_Angle))
  (bind _returnvalue (Transformation|GetWorldRotation _sm_ship))
  (if (Variables|HoverShip|GetTurn_On)
    (Transformation|SetWorldRotation (Variables|Default|GetSM_Ship) (Math|Rotator|MakeRotator (Math|Float|Clamp(Float) (.roll _returnvalue) (/ _min_rotation_angle 2.0) (/ _min_rotation_angle_2 2.0)) (Math|Float|Clamp(Float) (.pitch _returnvalue) _min_rotation_angle _min_rotation_angle_2) (.yaw _returnvalue)) false false)))

(fn CalculateMovementForce
  (bind _sm_ship (Variables|Default|GetSM_Ship))
  (bind _returnvalue (Physics|GetMass _sm_ship))
  (Variables|Movement|SetForwars_Force (* (* _returnvalue (Variables|Movement|GetForward_Accelaration)) 1e+02))
  (Variables|Movement|SetBackward_Force (* (* _returnvalue (Variables|Movement|GetBackward_Acceleration)) 1e+02))
  (Variables|Movement|SetTurn_Force (Math|Vector|VectorLength (* (Class|PrimitiveComponent|GetInertiaTensor (Variables|Default|GetSM_Ship) "None") (Variables|Movement|GetTurn_Acceleration)))))

(fn ApplyMovement
  (params (Move_Input :type Vector%202D%20Structure))
  (bind _forwars_force (Variables|Movement|GetForwars_Force))
  (Class|PrimitiveComponent|AddTorqueinRadians (Variables|Default|GetSM_Ship) (* (* (Math|Vector|GetUpVector (Variables|Default|GetSM_Ship)) (Variables|Movement|GetTurn_Force)) (.x Move_Input)) "None" false)
  (if (> (.y Move_Input) 0.0)
    (Physics|AddForce (Variables|Default|GetSM_Ship) (* (Math|Vector|GetForwardVector (Variables|Default|GetSM_Ship)) (Math|Float|SelectFloat _forwars_force (/ _forwars_force 5.0) (Variables|HoverShip|GetIs_Grounded?))) "None" false)
    (else
      (Physics|AddForce (Variables|Default|GetSM_Ship) (* (* (Math|Vector|GetForwardVector (Variables|Default|GetSM_Ship)) -1.0) (Variables|Movement|GetBackward_Force)) "None" false))))