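; Player-driven physics hover car that floats on four corner boosters, with throttle input only; steering is an empty stub.
; Each tick, a downward trace per booster applies a spring-like force to the Box, stronger nearer the ground.
; Grounded boosters also push forward by smoothed, decaying throttle input and shift the center of mass with it.
; Tick also restarts a camera shake every frame and computes an Acceleration value that is always zero.
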(event Input|EnhancedActionEvents|EnhancedInputActionIA_Accelerate
  (params (ActionValue :type Float%20%28double-precision%29) (ElapsedSeconds :type Float%20%28double-precision%29) (TriggeredSeconds :type Float%20%28double-precision%29) (InputAction :type Input%20Action%20Object%20Reference :default "/Game/Inputs/IA_Accelerate.IA_Accelerate"))
  (Variables|Default|SetAcceleration%20Input (Math|Interpolation|FInterpTo (Variables|Default|GetAcceleration%20Input) ActionValue (Utilities|Time|GetWorldDeltaSeconds) 0.5)))

(event Input|EnhancedActionEvents|EnhancedInputActionIA_Steer
  (params (ActionValue :type Float%20%28double-precision%29) (ElapsedSeconds :type Float%20%28double-precision%29) (TriggeredSeconds :type Float%20%28double-precision%29) (InputAction :type Input%20Action%20Object%20Reference :default "/Game/Inputs/IA_Steer.IA_Steer")))

(event EventBeginPlay
  (Input|AddMappingContext (PlayerController|LocalPlayerSubsystems|GetEnhancedInputLocalPlayerSubsystem (Game|GetPlayerController 0)) "/Game/Inputs/IC_Vehicle.IC_Vehicle" 0 "(bIgnoreAllPressedKeysUntilRelease=True,bForceImmediately=False,bNotifyUserSettings=False)"))

(event Collision|EventActorBeginOverlap
  (params (OtherActor :type Actor%20Object%20Reference)))

(event EventTick
  (params (DeltaSeconds :type Float%20%28single-precision%29))
  (CallFunction|SuspensionCast (Variables|Default|GetFL_Booster))
  (CallFunction|SuspensionCast (Variables|Default|GetFR_Booster))
  (CallFunction|SuspensionCast (Variables|Default|GetBR_Booster))
  (CallFunction|SuspensionCast (Variables|Default|GetBL_Booster))
  (CallFunction|CalculateAcceleration)
  (Game|Feedback|ClientStartCameraShake (Game|GetPlayerController 0) "/Game/Blueprints/Shake.Shake_C" 1.0 "World" "0, 0, 0"))

(fn ConstructionScript)

(fn SuspensionCast
  (params (Wheel%20Comp :type Scene%20Component%20Object%20Reference))
  (bind _returnvalue (Transformation|GetWorldLocation Wheel%20Comp))
  (bind _outhit (Collision|LineTraceByChannel _returnvalue (+ _returnvalue (* (Math|Vector|GetUpVector Wheel%20Comp) -6e+01)) "TraceTypeQuery1" false 0 "ForOneFrame"))
  (if (.bBlockingHit (Collision|BreakHitResult _outhit))
    (Class|PrimitiveComponent|AddForceatLocation (Variables|Default|GetBox) (* (- 1.0 (Math|Float|NormalizetoRange (.Distance (Collision|BreakHitResult _outhit)) 0.0 6e+01)) (Math|Vector|GetUnitDirection(Vector) (.TraceEnd (Collision|BreakHitResult _outhit)) (.TraceStart (Collision|BreakHitResult _outhit))) 1e+05) (Transformation|GetWorldLocation Wheel%20Comp) "None")
    (CallFunction|AccelerateCar Wheel%20Comp)))

(fn CalculateAcceleration
  (Variables|Default|SetAcceleration (* 0.0 (Variables|Default|GetAcceleration%20Input)))
  (Variables|Default|SetAcceleration%20Input (Math|Interpolation|FInterpTo (Variables|Default|GetAcceleration%20Input) 0.0 (Utilities|Time|GetWorldDeltaSeconds) 0.4)))

(fn AccelerateCar
  (params (Wheel%20Comp :type Scene%20Component%20Object%20Reference))
  (bind _box (Variables|Default|GetBox))
  (Class|PrimitiveComponent|AddForceatLocation (Variables|Default|GetBox) (* (Math|Vector|GetForwardVector _box) 1e+03 (Variables|Default|GetAcceleration%20Input) (Physics|GetMass _box)) (Transformation|GetWorldLocation Wheel%20Comp) "None")
  (Class|PrimitiveComponent|SetCenterOfMass (Variables|Default|GetBox) (* "100.000000,0.000000,0.000000" (Variables|Default|GetAcceleration%20Input)) "None"))